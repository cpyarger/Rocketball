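; BP_BlueGate is the blue end of a teleport gate pair, sending the player to BP_RedGate.
; When a FirstPersonCharacter overlaps its box, it teleports player pawn 0 to the first red gate's location and rotation.
; The character's IsTeleporting flag guards against bouncing back: it is set on departure, and an overlap while it is set only clears it after a short delay.
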(event `self.Box.OnComponentBeginOverlap`
  (params (OverlappedComponent :type "PrimitiveComponent Object Reference") (OtherActor :type "Actor Object Reference") (OtherComp :type "PrimitiveComponent Object Reference") (OtherBodyIndex :type Integer) (bFromSweep :type Boolean) (SweepResult :type "HitResult Structure (by ref)"))
  (bind _asfirst_person_character (cast `/Game/FirstPersonBP/Blueprints/FirstPersonCharacter` OtherActor))
  (if (`/Game/FirstPersonBP/Blueprints/FirstPersonCharacter.IsTeleporting?` _asfirst_person_character)
    (`KismetSystemLibrary.Delay` 0.5)
    (set `/Game/FirstPersonBP/Blueprints/FirstPersonCharacter.IsTeleporting?` false _asfirst_person_character)
    (else
      (bind _outactors (`GameplayStatics.GetAllActorsOfClass` "/Game/RocketBall/Gate/BP_RedGate.BP_RedGate_C"))
      (set `/Game/FirstPersonBP/Blueprints/FirstPersonCharacter.IsTeleporting?` true _asfirst_person_character)
      (bind _item (`KismetArrayLibrary.Array_Get` _outactors))
      (`self.K2_SetActorLocationAndRotation` (`GameplayStatics.GetPlayerPawn` 0) (`self.K2_GetActorLocation` _item) (`self.K2_GetActorRotation` _item) false true))))

(fn `UserConstructionScript`)